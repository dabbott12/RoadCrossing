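; Player Blueprint for a step-based movement game that hops forward, left or right in fixed increments and owns the score and game-over UI.
; Input calls TryMove, which shifts a target position and locks movement until a short timer re-enables it.
; Tick drives the root component toward that target with MoveComponentTo.
; BeginPlay creates the score widget, AddScore updates it, and GameOver shows the end screen and mouse cursor.
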(event `InputAction|Move_Forward`
  (params (Key :type "Key Structure"))
  ;[1 1 1] Movement Control
  (:`Pressed`
    (`self.TryMove` (100.0 0.0 0.0))))

(event `InputAction|Move_Left`
  (params (Key :type "Key Structure"))
  ;[1 1 1] Movement Control
  (:`Pressed`
    (`self.TryMove` (0.0 -100.0 0.0))))

(event `InputAction|Move_Right`
  (params (Key :type "Key Structure"))
  ;[1 1 1] Movement Control
  (:`Pressed`
    (`self.TryMove` (0.0 100.0 0.0))))

(event `self.ReceiveTick`
  (params (DeltaSeconds :type "Float (single-precision)"))
  ;[1 1 1] Actual Movement
  (`KismetSystemLibrary.MoveComponentTo` (`self.DefaultSceneRoot`) (`self.TargetPosition`)))

(event `self.ReceiveBeginPlay`
  ;[1 1 1] Creates Score UI
  (bind _returnvalue (`|CreateWidget` "/Game/Blueprints/ScoreUI.ScoreUI_C"))
  (`UserWidget.AddToViewport` _returnvalue 0)
  (bind _output_get (set `self.ScoreUI` _returnvalue))
  (`/Game/Blueprints/ScoreUI.UpdateScoreText` _output_get (`self.Score`)))

(fn `AddScore`
  (params (ScoreToAdd :type Integer))
  (bind _output_get (set `self.Score` (+ ScoreToAdd (`self.Score`))))
  (`/Game/Blueprints/ScoreUI.UpdateScoreText` (`self.ScoreUI`) _output_get))

(fn `EnableCanMove`
  (set `self.CanMove` true))

(fn `GameOver`
  (bind _returnvalue (`|CreateWidget` "/Game/Blueprints/EndSceneUI.EndSceneUI_C"))
  (`UserWidget.AddToViewport` _returnvalue 0)
  (`/Game/Blueprints/EndSceneUI.SetGameOverScreen` _returnvalue)
  (set `PlayerController.bShowMouseCursor` true (`GameplayStatics.GetPlayerController` 0)))

(fn `TryMove`
  (params (Direction :type "Vector Structure"))
  (if (`self.CanMove`)
    (set `self.TargetPosition` (+ Direction (`self.TargetPosition`)))
    (set `self.CanMove` false)
    (`KismetSystemLibrary.K2_SetTimer` null "EnableCanMove" 0.3)))

(fn `UserConstructionScript`)