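; Car is an obstacle actor that drives along its root component's forward vector and ends the game when it hits the player.
; Each Tick offsets it by Speed scaled by delta time, without sweep, and snaps it back to StartPosition once it travels beyond Distance, creating a loop.
; Actor overlap casts the other actor to Player and calls GameOver on it.
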(event `self.ReceiveTick`
  (params (DeltaSeconds :type "Float (single-precision)"))
  ;[1 1 1] Movement
  (`self.K2_AddActorWorldOffset` (* (`SceneComponent.GetForwardVector` (`self.DefaultSceneRoot`)) (* DeltaSeconds (`self.Speed`))))
  (if (> (`KismetMathLibrary.Vector_Distance` (`self.K2_GetActorLocation`) (`self.StartPosition`)) (`self.Distance`))
    (`self.K2_SetActorLocation` (`self.StartPosition`))))

(event `self.ReceiveActorBeginOverlap`
  (params (OtherActor :type "Actor Object Reference"))
  ;[1 1 1] Collision For Player
  (bind _asplayer (cast `/Game/Blueprints/Player` OtherActor))
  (`/Game/Blueprints/Player.GameOver` _asplayer))

(fn `UserConstructionScript`)